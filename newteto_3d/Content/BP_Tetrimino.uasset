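; BP_Tetrimino is a tetrimino actor that builds its block grid from static mesh components at runtime.
; BeginPlay loops over 16 indices, using integer division and modulo by 4 to place a mesh on a 4x4 grid with 100-unit spacing.
; The branch is fixed to true, so every cell gets a block; the TetriminoData shape check and debug prints are left unconnected.
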(event EventBeginPlay
  (for _index (range 0 15)
    (if true
      (AddComponent|AddStaticMeshComponent false (Math|Transform|MakeTransform (Math|Vector|MakeVector (Math|Conversions|ToFloat(Integer) (* (Math|Float|Floor (Math|Conversions|ToFloat(Integer) (/ _index 4))) 100)) (Math|Conversions|ToFloat(Integer) (* (Math|Float|Floor (Math|Conversions|ToFloat(Integer) (Math|Integer|%(Integer) _index 4))) 100)) 0.0) "0, 0, 0" "1.000000,1.000000,1.000000")))))

(event Collision|EventActorBeginOverlap
  (params (OtherActor :type Actor%20Object%20Reference)))

(event EventTick
  (params (DeltaSeconds :type Float%20%28single-precision%29)))

(fn ConstructionScript)